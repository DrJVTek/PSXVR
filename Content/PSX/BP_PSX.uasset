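; BP_PSX hosts an R3000 PlayStation emulator in Unreal, set up to boot a Ridge Racer disc image from hardcoded local paths.
; On BeginPlay it configures and initializes the emulator component, printing BIOS output to screen through a bound event.
; It then gives the GPU component a polygon base material and a placed VRAM viewer.
; Tick does nothing, and the step-count logging is disconnected.
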(event Custom|CustomEvent
  (params (Line :type String))
  (Development|PrintText (Utilities|Text|ToText(String) Line) true true "(R=0.053789,G=0.187500,B=0.029930,A=1.000000)"))

(event EventBeginPlay
  (bind _r3000emu (Variables|Default|GetR3000Emu))
  (bind _r3000gpu (Variables|Default|GetR3000Gpu))
  (Utilities|FlowControl|Sequence
    (:then_0
      (Variables|/Script/R3000EmuRuntime.R3000EmuComponent|SetBiosPath _r3000emu "E:\\Projects\\github\\Live\\R3000-Emu\\bios\\ps1_bios.bin")
      (Variables|/Script/R3000EmuRuntime.R3000EmuComponent|SetDiscPath _r3000emu "E:\\Projects\\PSX\\roms\\Ridge Racer (U).cue")
      (Variables|/Script/R3000EmuRuntime.R3000EmuComponent|SetOutputDir _r3000emu "E:\\Projects\\github\\Live\\PSXVR\\logs")
      (Variables|/Script/R3000EmuRuntime.R3000EmuComponent|SetbRunning _r3000emu true)
      (Variables|/Script/R3000EmuRuntime.R3000EmuComponent|SetEmuLogLevel _r3000emu "trace")
      (Variables|/Script/R3000EmuRuntime.R3000EmuComponent|SetCoreLogLevel _r3000emu "warn")
      (Variables|/Script/R3000EmuRuntime.R3000EmuComponent|SetbTraceASM _r3000emu false)
      (Variables|/Script/R3000EmuRuntime.R3000EmuComponent|SetbTraceIO _r3000emu false)
      (Variables|/Script/R3000EmuRuntime.R3000EmuComponent|SetBudgetMs _r3000emu 5e+01)
      (Variables|/Script/R3000EmuRuntime.R3000EmuComponent|SetCoreLogCats _r3000emu "exc")
      (Class|R3000EmuComponent|InitEmulator _r3000emu)
      (EventDispatchers|BindEventtoOnBiosPrint _r3000emu (delegate Custom|CustomEvent)))
    (:then_1
      (Variables|/Script/R3000EmuRuntime.R3000GpuComponent|SetVramViewerMaterial _r3000gpu "/Game/PSX/M_VramViewer.M_VramViewer")
      (Variables|/Script/R3000EmuRuntime.R3000GpuComponent|SetVramViewerOffset _r3000gpu "0.000000,800.000000,-100.000000")
      (Variables|/Script/R3000EmuRuntime.R3000GpuComponent|SetVramViewerRotation _r3000gpu "0, 0, 0")
      (Variables|/Script/R3000EmuRuntime.R3000GpuComponent|SetVramViewerScale _r3000gpu 0.5)
      (Variables|/Script/R3000EmuRuntime.R3000GpuComponent|SetBaseMaterial _r3000gpu "/Game/PSX/M_PlayPoly.M_PlayPoly")
      (Development|PrintText "Init OK" true true "(R=0.053789,G=0.187500,B=0.029930,A=1.000000)"))))

(event EventTick
  (params (DeltaSeconds :type Float%20%28single-precision%29)))

(fn ConstructionScript)